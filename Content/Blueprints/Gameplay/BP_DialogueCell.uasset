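; Dialogue actor that runs a conversation between the player pawn's widget and its BPCDialogueComponent, which supplies row-based dialogue data.
; Activate picks a first or second start row based on whether a dialogue flag is set, then displays the line and any choices.
; Update records the first obtained flag, then advances rows or exits the dialogue.
; Selecting one of two choices triggers its GameInstance effect and jumps to that choice's next row.
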(event Custom|OnChoicesSelected
  (params (ChoiceIndex :type Integer))
  (bind _bpc_dialoguecomponent (Variables|Default|GetBPC_DialogueComponent))
  (bind _bpc_dialoguecomponent_2 (Variables|Default|GetBPC_DialogueComponent))
  (bind (_haschoice _choice1text _choice1nextrow _choice1effect _choice2text _choice2nextrow _choice2effect) (Default|GetChoiceData (Variables|Default|GetBPC_DialogueComponent)))
  (switch int ChoiceIndex
    (:0
      (Default|TriggerEffect (Variables|Default|GetGameInstanceRef) _choice1effect)
      (Variables|/Game/Blueprints/Global/BPC_DialogueComponent.BPC_DialogueComponent_C|SetCurrentRowNumber _bpc_dialoguecomponent _choice1nextrow)
      (Default|GetCurrentDialogueRowData _bpc_dialoguecomponent)
      (bind _charactername (Default|GetCharacterfromCurrentRow _bpc_dialoguecomponent))
      (bind _dialoguelong (Default|GetDialogueLongfromCurrentRow _bpc_dialoguecomponent))
      (Default|UpdateDialogue (Variables|/Game/Blueprints/Gameplay/BP_Pawn.BP_Pawn_C|GetWidget (Variables|Default|GetPlayerRef)) _charactername _dialoguelong))
    (:1
      (Default|TriggerEffect (Variables|Default|GetGameInstanceRef) _choice2effect)
      (Variables|/Game/Blueprints/Global/BPC_DialogueComponent.BPC_DialogueComponent_C|SetCurrentRowNumber _bpc_dialoguecomponent_2 _choice2nextrow)
      (Default|GetCurrentDialogueRowData _bpc_dialoguecomponent_2)
      (bind _charactername_2 (Default|GetCharacterfromCurrentRow _bpc_dialoguecomponent_2))
      (bind _dialoguelong_2 (Default|GetDialogueLongfromCurrentRow _bpc_dialoguecomponent_2))
      (Default|UpdateDialogue (Variables|/Game/Blueprints/Gameplay/BP_Pawn.BP_Pawn_C|GetWidget (Variables|Default|GetPlayerRef)) _charactername_2 _dialoguelong_2))))

(event EventBeginPlay
  (|CallParentFunction))

(event Collision|EventActorBeginOverlap
  (params (OtherActor :type Actor%20Object%20Reference))
  (|CallParentFunction OtherActor) ; This node is disabled and will not be called.\nDrag off pins to build functionality.
)

(event EventTick
  (params (DeltaSeconds :type Float%20%28single-precision%29))
  (|CallParentFunction DeltaSeconds) ; This node is disabled and will not be called.\nDrag off pins to build functionality.
)

(event EventActivate
  (params (Pawn :type BP%20Pawn%20Object%20Reference))
  (bind _bpc_dialoguecomponent (Variables|Default|GetBPC_DialogueComponent))
  (bind _widget (Variables|/Game/Blueprints/Gameplay/BP_Pawn.BP_Pawn_C|GetWidget Pawn))
  (Variables|Default|SetPlayerRef Pawn)
  (bind _startrow (CallFunction|DetermineStartRow))
  (Variables|/Game/Blueprints/Global/BPC_DialogueComponent.BPC_DialogueComponent_C|SetCurrentRowNumber _bpc_dialoguecomponent _startrow)
  (Default|GetCurrentDialogueRowData _bpc_dialoguecomponent)
  (bind _charactername (Default|GetCharacterfromCurrentRow _bpc_dialoguecomponent))
  (bind _dialoguelong (Default|GetDialogueLongfromCurrentRow _bpc_dialoguecomponent))
  (Variables|/Game/Blueprints/Global/Widget/WBP_DialogueUI.WBP_DialogueUI_C|SetDialogueCellRef _widget self)
  (Default|UpdateDialogue _widget _charactername _dialoguelong)
  (Default|StartDialogue _widget)
  (bind (_haschoice _choice1text _choice1nextrow _choice1effect _choice2text) (Default|GetChoiceData (Variables|Default|GetBPC_DialogueComponent)))
  (if _haschoice
    (Default|ShowChoices _widget _choice1text _choice2text)
    (else
      (Default|HideChoices _widget))))

(event EventUpdate
  (params (Pawn :type BP%20Pawn%20Object%20Reference))
  (bind _bpc_dialoguecomponent (Variables|Default|GetBPC_DialogueComponent))
  (bind _bpc_dialoguecomponent_2 (Variables|Default|GetBPC_DialogueComponent))
  (bind _widget (Variables|/Game/Blueprints/Gameplay/BP_Pawn.BP_Pawn_C|GetWidget Pawn))
  (bind _flagobtains (Variables|/Game/Blueprints/Global/BPC_DialogueComponent.BPC_DialogueComponent_C|GetFlagObtains _bpc_dialoguecomponent))
  (if (> (Utilities|Array|Length _flagobtains) 0)
    (Variables|Default|SetDialogueFlagName (Utilities|Array|Get(acopy) _flagobtains)))
  (bind _bisfinished (Default|IsDialogueFinished _bpc_dialoguecomponent_2))
  (if _bisfinished
    (Default|ExitDialogue _widget)
    (Default|HideChoices _widget)
    (else
      (Default|ReadNextRow _bpc_dialoguecomponent_2)
      (bind _charactername (Default|GetCharacterfromCurrentRow _bpc_dialoguecomponent_2))
      (bind _dialoguelong (Default|GetDialogueLongfromCurrentRow _bpc_dialoguecomponent_2))
      (bind (_haschoice _choice1text _choice1nextrow _choice1effect _choice2text) (Default|GetChoiceData (Variables|Default|GetBPC_DialogueComponent)))
      (if _haschoice
        (Default|ShowChoices _widget _choice1text _choice2text)
        (else
          (Default|UpdateDialogue _widget _charactername _dialoguelong))))))

(fn ConstructionScript
  (|CallParentFunction))

(fn DetermineStartRow
  (bind _seconddialgouestartrow (Variables|Default|GetSecondDialgoueStartRow))
  (if (!= (Variables|Default|GetDialogueFlagName) "")
    (Development|PrintString (Utilities|String|ToString(Integer) _seconddialgouestartrow))
    (return _seconddialgouestartrow)
    (else
      (return (Variables|Default|GetFirstDialogueStartRow)))))