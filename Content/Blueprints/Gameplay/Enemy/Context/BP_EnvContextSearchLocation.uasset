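; EQS context that supplies search locations and a reference actor to environment queries for the hide-and-seek enemy AI.
; The location set comes from SearchedLocation on the querier's BP_AI_HideAndSeek controller, falling back to DebugLocation when that cast fails.
; The single-actor provider returns the player pawn, or the first PlayerStart found when no valid pawn exists.
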(fn ProvideSingleActor
  (params (QuerierObject :type Object%20Object%20Reference) (QuerierActor :type Actor%20Object%20Reference))
  (bind _returnvalue (Game|Player|GetPlayerPawn 0))
  (if (Utilities|IsValid _returnvalue)
    (return _returnvalue)
    (else
      (bind _outactors (Actor|GetAllActorsOfClass "/Script/Engine.PlayerStart"))
      (return (Utilities|Array|Get(acopy) _outactors)))))

(fn ProvideLocationsSet
  (params (QuerierObject :type Object%20Object%20Reference) (QuerierActor :type Actor%20Object%20Reference))
  (bind _asbp_ai_hide_and_seek (Utilities|Casting|CastToBP_AI_HideAndSeek (AI|GetAIController QuerierActor))
    (:then
      (return (Variables|/Game/Blueprints/Gameplay/Enemy/BP_AI_HideAndSeek.BP_AI_HideAndSeek_C|GetSearchedLocation%20 _asbp_ai_hide_and_seek)))
    (:CastFailed
      (return (LocalVariables|GetDebugLocation)))))