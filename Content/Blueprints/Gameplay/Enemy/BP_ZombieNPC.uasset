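; BP_ZombieNPC is an enemy for a hide-and-seek minigame, driven by the BP_AI_HideAndSeek controller.
; On BeginPlay it copies its IsHiding role to that controller.
; Detection and lose spheres set and clear PlayerDetected as the player enters one and leaves the other.
; When the player overlaps a third sphere and the zombie is not hiding, it calls GameFinished on the BP_MiniGameManager.
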(event OnComponentBeginOverlap(DetectionSphere)
  (params (OverlappedComponent :type Primitive%20Component%20Object%20Reference) (OtherActor :type Actor%20Object%20Reference) (OtherComp :type Primitive%20Component%20Object%20Reference) (OtherBodyIndex :type Integer) (bFromSweep :type Boolean) (SweepResult :type Hit%20Result%20Structure%20%28by%20ref%29))
  (if (== OtherActor (Game|Player|GetPlayerPawn 0))
    (Variables|Default|SetPlayerDetected true)
    (if true
      _)))

(event OnComponentEndOverlap(LoseSphere)
  (params (OverlappedComponent :type Primitive%20Component%20Object%20Reference) (OtherActor :type Actor%20Object%20Reference) (OtherComp :type Primitive%20Component%20Object%20Reference) (OtherBodyIndex :type Integer))
  (if (== OtherActor (Game|Player|GetPlayerPawn 0))
    (bind _output_get (Variables|Default|SetPlayerDetected false))
    (Development|PrintString (Utilities|String|ToString(Boolean) _output_get))))

(event OnComponentBeginOverlap(Sphere)
  (params (OverlappedComponent :type Primitive%20Component%20Object%20Reference) (OtherActor :type Actor%20Object%20Reference) (OtherComp :type Primitive%20Component%20Object%20Reference) (OtherBodyIndex :type Integer) (bFromSweep :type Boolean) (SweepResult :type Hit%20Result%20Structure%20%28by%20ref%29))
  (if (== OtherActor (Game|Player|GetPlayerPawn 0))
    (if (not (Variables|Default|GetIsHiding?))
      (bind _returnvalue (Actor|GetActorOfClass "/Game/Blueprints/Global/BP_MiniGameManager.BP_MiniGameManager_C"))
      (Default|GameFinished _returnvalue 2))))

(event EventBeginPlay
  (bind _asbp_ai_hide_and_seek (Utilities|Casting|CastToBP_AI_HideAndSeek (Pawn|GetController)))
  (Variables|/Game/Blueprints/Gameplay/Enemy/BP_AI_HideAndSeek.BP_AI_HideAndSeek_C|SetIsHiding _asbp_ai_hide_and_seek (Variables|Default|GetIsHiding?)))

(event Collision|EventActorBeginOverlap
  (params (OtherActor :type Actor%20Object%20Reference)))

(event EventTick
  (params (DeltaSeconds :type Float%20%28single-precision%29)))

(fn ConstructionScript)