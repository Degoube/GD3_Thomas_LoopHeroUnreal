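; BP_TrapCell is a trap cell that costs the player gold when activated.
; Its Activate event casts the game instance to BP_LoopGameInstance and subtracts a small random amount from PlayerGold, clamped so it never drops below zero.
; BeginPlay, overlap and Tick are disabled stubs, and the construction script only calls its parent.
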(event EventBeginPlay
  (|CallParentFunction) ; This node is disabled and will not be called.\nDrag off pins to build functionality.
)

(event Collision|EventActorBeginOverlap
  (params (OtherActor :type Actor%20Object%20Reference))
  (|CallParentFunction OtherActor) ; This node is disabled and will not be called.\nDrag off pins to build functionality.
)

(event EventTick
  (params (DeltaSeconds :type Float%20%28single-precision%29))
  (|CallParentFunction DeltaSeconds) ; This node is disabled and will not be called.\nDrag off pins to build functionality.
)

(event EventActivate
  (params (Pawn :type BP%20Pawn%20Object%20Reference))
  (bind _asbp_loop_game_instance (Utilities|Casting|CastToBP_LoopGameInstance (Game|GetGameInstance)))
  (Variables|/Game/Blueprints/Global/BP_LoopGameInstance.BP_LoopGameInstance_C|SetPlayerGold _asbp_loop_game_instance (Math|Integer|Max(Integer) (- (Variables|/Game/Blueprints/Global/BP_LoopGameInstance.BP_LoopGameInstance_C|GetPlayerGold _asbp_loop_game_instance) (Math|Random|RandomIntegerinRange 5 15)))))

(fn ConstructionScript
  (|CallParentFunction))