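; BP_Shooter is an activatable actor that sends the player into the "Shooter" level.
; On Activate it disables the pawn's input, starts a WBP_BlackScreen fade-out, saves through BP_LoopGameInstance and opens the level.
; The save and level load run immediately rather than waiting for the fade, whose finished callback only removes the widget.
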(event Custom|FadeOutDone
  (Widget|RemovefromParent (stale EventActivate _returnvalue)))

(event EventBeginPlay
  (|CallParentFunction) ; This node is disabled and will not be called.\nDrag off pins to build functionality.
)

(event Collision|EventActorBeginOverlap
  (params (OtherActor :type Actor%20Object%20Reference))
  (|CallParentFunction OtherActor) ; This node is disabled and will not be called.\nDrag off pins to build functionality.
)

(event EventTick
  (params (DeltaSeconds :type Float%20%28single-precision%29))
  (|CallParentFunction DeltaSeconds) ; This node is disabled and will not be called.\nDrag off pins to build functionality.
)

(event EventActivate
  (params (Pawn :type BP%20Pawn%20Object%20Reference))
  (Input|DisableInput Pawn (Game|GetPlayerController 0))
  (bind _returnvalue (UserInterface|CreateWidget "/Game/Blueprints/Global/Widget/WBP_BlackScreen.WBP_BlackScreen_C"))
  (UserInterface|Viewport|AddtoViewport _returnvalue 100)
  (Default|PlayFadeOut _returnvalue)
  (EventDispatchers|BindEventtoOnFadeFinished _returnvalue (delegate Custom|FadeOutDone))
  (bind _asbp_loop_game_instance (Utilities|Casting|CastToBP_LoopGameInstance (Game|GetGameInstance)))
  (Default|SaveGametoSlot _asbp_loop_game_instance)
  (Game|OpenLevel(byName) "Shooter"))

(fn ConstructionScript
  (|CallParentFunction))