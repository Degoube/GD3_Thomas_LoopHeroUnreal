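; Board-game pawn that moves between cells by dice steps and triggers the message of the cell it occupies.
; On BeginPlay it creates the dialogue UI, links it to the dice and itself, and activates the current cell.
; StartMove stores the target cell in the game instance, then a timeline lerps the pawn there and activates it.
; A separate OnStepComplete event checks lap progress and opens the Win or Lose level.
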(event Custom|StartMove
  (params (Steps :type Integer))
  (bind _bp_loop_game_instance (Variables|Default|GetBP%20Loop%20Game%20Instance))
  (bind _cell (Default|GetNextCelltoMove (Variables|Default|GetBoard) (+ Steps (Variables|/Game/Blueprints/Global/BP_LoopGameInstance.BP_LoopGameInstance_C|Get%20CellNumber _bp_loop_game_instance))))
  (bind _output_get (Variables|/Game/Blueprints/Global/BP_LoopGameInstance.BP_LoopGameInstance_C|Set%20CellNumber _bp_loop_game_instance _cell))
  (bind _cell_2 (Default|GetCellbyNumber (Variables|Default|GetBoard) _output_get))
  (Variables|Default|SetTargetLocation%20 (Transformation|GetActorLocation _cell_2))
  (Variables|Default|SetStartLocation (Transformation|GetActorLocation))
  (bind _alpha (Timeline|Tl_Move PlayFromStart)
    (:Update
      (Transformation|SetActorLocation (Math|Vector|Lerp(Vector) (Variables|Default|GetStartLocation) (+ (Variables|Default|GetTargetLocation%20) "0.000000,0.000000,95.000000") _alpha) false false))
    (:Finished
      (CallFunction|ActivateCell))))

(event Custom|OnStepComplete
  (bind _bp_loop_game_instance (Variables|Default|GetBP%20Loop%20Game%20Instance))
  (bind _currentturn (Variables|/Game/Blueprints/Global/BP_LoopGameInstance.BP_LoopGameInstance_C|GetCurrentTurn _bp_loop_game_instance))
  (Variables|Default|SetIsMoving false)
  (CallFunction|ActivateCell)
  (if (>= (Variables|/Game/Blueprints/Global/BP_LoopGameInstance.BP_LoopGameInstance_C|Get%20CellNumber _bp_loop_game_instance) (* 16 _currentturn))
    (bind _result (Math|Integer|IncrementInt _currentturn)
      (:%20%20
        (if (> _result (Variables|/Game/Blueprints/Global/BP_LoopGameInstance.BP_LoopGameInstance_C|GetMaxTurn _bp_loop_game_instance))
          (Game|OpenLevel(byName) "Win")
          (else
            (Game|OpenLevel(byName) "Lose")))))))

(event EventBeginPlay
  (bind _asbp_loop_game_instance (Utilities|Casting|CastToBP_LoopGameInstance (Game|GetGameInstance)))
  (Variables|Default|SetBP%20Loop%20Game%20Instance _asbp_loop_game_instance)
  (bind _returnvalue (UserInterface|CreateWidget "/Game/Blueprints/Global/Widget/WBP_DialogueUI.WBP_DialogueUI_C" (Game|GetPlayerController 0) 0))
  (bind _output_get (Variables|Default|SetWidget _returnvalue))
  (Variables|/Game/Blueprints/Global/Widget/WBP_DialogueUI.WBP_DialogueUI_C|SetDice _output_get (Variables|Default|GetDice))
  (Variables|/Game/Blueprints/Global/Widget/WBP_DialogueUI.WBP_DialogueUI_C|SetPawn _output_get self)
  (UserInterface|Viewport|AddtoViewport _output_get 0)
  ;[0.15 0.15 0.15 0.5] Penser à le retirer
  (CallFunction|ActivateCell))

(fn ConstructionScript)

(fn ActivateCell
  (bind _cell (Default|GetCellbyNumber (Variables|Default|GetBoard) (Variables|/Game/Blueprints/Global/BP_LoopGameInstance.BP_LoopGameInstance_C|Get%20CellNumber (Variables|Default|GetBP%20Loop%20Game%20Instance))))
  (Class|BPIActivable|Activate(Message) _cell self))

(fn UpdateCell
  (bind _cell (Default|GetCellbyNumber (Variables|Default|GetBoard) (Variables|/Game/Blueprints/Global/BP_LoopGameInstance.BP_LoopGameInstance_C|Get%20CellNumber (Variables|Default|GetBP%20Loop%20Game%20Instance))))
  (Class|BPIActivable|Update(Message) _cell self))