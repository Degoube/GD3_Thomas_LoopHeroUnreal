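; Game instance that holds the player's gold, keys, cell, turn counters and dialogue flags, with save, load and delete on the "LoopSave" slot.
; Init attempts a load and writes a fresh BP_LoopSave if that fails.
; TriggerEffect adjusts gold or keys, opening the Lose level when a gold loss reaches zero.
; LoadGameFromSlot copies instance values onto the loaded object, so saved values never reach the instance.
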(event EventInit
  (bind _sucess (CallFunction|LoadGamefromSlot))
  (if (not _sucess)
    (CallFunction|SaveGametoSlot)))

(fn SetFlag
  (params (FlagName :type Name))
  (Utilities|Map|Add (Variables|Default|GetDialogueFlags) FlagName true))

(fn GetFlag
  (params (Flag :type Name))
  (bind _dialogueflags (Variables|Default|GetDialogueFlags))
  (bind (_value _returnvalue) (Utilities|Map|Find _dialogueflags Flag))
  (Development|PrintString (Utilities|String|ToString(Boolean) _value))
  (return _returnvalue))

(fn TriggerEffect
  (params (Effect :type Name))
  (switch name Effect
    (:GiveGold
      (Variables|Default|SetPlayerGold (+ (Variables|Default|GetPlayerGold) 15)))
    (:GiveKey
      (Variables|Default|SetPlayerKeys (+ (Variables|Default|GetPlayerKeys) 1)))
    (:LoseGold
      (bind _output_get (Variables|Default|SetPlayerGold (Math|Integer|Max(Integer) (- (Variables|Default|GetPlayerGold) 10))))
      (if (<= _output_get 0)
        (Game|OpenLevel(byName) "Lose")))))

(fn SaveGametoSlot
  (bind _returnvalue (SaveGame|CreateSaveGameObject "/Game/Blueprints/Global/BP_LoopSave.BP_LoopSave_C"))
  (bind _output_get (LocalVariables|SetSaveData _returnvalue))
  (Variables|/Game/Blueprints/Global/BP_LoopSave.BP_LoopSave_C|SetPlayerKeys _output_get (Variables|Default|GetPlayerKeys))
  (Variables|/Game/Blueprints/Global/BP_LoopSave.BP_LoopSave_C|SetPlayerGold _output_get (Variables|Default|GetPlayerGold))
  (Variables|/Game/Blueprints/Global/BP_LoopSave.BP_LoopSave_C|Set%20CellNumber _output_get (Variables|Default|Get%20CellNumber))
  (Variables|/Game/Blueprints/Global/BP_LoopSave.BP_LoopSave_C|SetMaxTurn _output_get (Variables|Default|GetMaxTurn))
  (Variables|/Game/Blueprints/Global/BP_LoopSave.BP_LoopSave_C|SetCurrentTurn _output_get (Variables|Default|GetCurrentTurn))
  (Variables|/Game/Blueprints/Global/BP_LoopSave.BP_LoopSave_C|SetDialogueFlags _output_get (Variables|Default|GetDialogueFlags))
  (SaveGame|SaveGametoSlot (LocalVariables|GetSaveData) "LoopSave"))

(fn LoadGamefromSlot
  (bind _returnvalue (SaveGame|DoesSaveGameExist "LoopSave"))
  (if _returnvalue
    (bind _returnvalue_2 (SaveGame|LoadGamefromSlot "LoopSave"))
    (bind _asbp_loop_save (Utilities|Casting|CastToBP_LoopSave _returnvalue_2)
      (:then
        (Variables|/Game/Blueprints/Global/BP_LoopSave.BP_LoopSave_C|Set%20CellNumber _asbp_loop_save (Variables|Default|Get%20CellNumber))
        (Variables|/Game/Blueprints/Global/BP_LoopSave.BP_LoopSave_C|SetCurrentTurn _asbp_loop_save (Variables|Default|GetCurrentTurn))
        (Variables|/Game/Blueprints/Global/BP_LoopSave.BP_LoopSave_C|SetPlayerKeys _asbp_loop_save (Variables|Default|GetPlayerKeys))
        (Variables|/Game/Blueprints/Global/BP_LoopSave.BP_LoopSave_C|SetPlayerGold _asbp_loop_save (Variables|Default|GetPlayerGold))
        (Variables|/Game/Blueprints/Global/BP_LoopSave.BP_LoopSave_C|SetDialogueFlags _asbp_loop_save (Variables|Default|GetDialogueFlags))
        (return true))
      (:CastFailed
        (return false)))
    (else
      (return false))))

(fn DeleteSaveGame
  (SaveGame|DeleteGameinSlot "LoopSave"))