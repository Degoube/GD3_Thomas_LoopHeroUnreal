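; Dialogue component that steps through rows of a dialogue DataTable, tracking the current row by number.
; Loading a row caches it and, if it names a flag, sets that flag on BP_LoopGameInstance and records it in FlagObtains.
; Getters expose the row's text, character and two-option choice data.
; ReadNextRow follows the NextRow index; dialogue counts as finished when that index is negative and no choice exists.
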(fn GetCurrentDialogueRowData
  (bind _returnvalue (Utilities|GetDataTableRow (Variables|Default|GetDialogueDataTable) (Utilities|String|StringToName (Utilities|String|ToString(Integer) (Variables|Default|GetCurrentRowNumber))))
    (:then
      (bind _output_get (Variables|Default|SetCurrentDialogueRow _returnvalue))
      (if (!= (.SetsFlag (Utilities|Struct|BreakST_DialogueRowDatas _output_get)) "None")
        (bind _asbp_loop_game_instance (Utilities|Casting|CastToBP_LoopGameInstance (Game|GetGameInstance)))
        (Default|SetFlag _asbp_loop_game_instance (.SetsFlag (Utilities|Struct|BreakST_DialogueRowDatas _output_get)))
        (Utilities|Array|Add (Variables|Default|GetFlagObtains) (.SetsFlag (Utilities|Struct|BreakST_DialogueRowDatas _output_get))))
      (return _output_get))))

(fn GetDialogueLongfromCurrentRow
  (return (.DialogueLong (Utilities|Struct|BreakST_DialogueRowDatas (Variables|Default|GetCurrentDialogueRow)))))

(fn GetCharacterfromCurrentRow
  (return (.Character (Utilities|Struct|BreakST_DialogueRowDatas (Variables|Default|GetCurrentDialogueRow)))))

(fn IsDialogueFinished
  (bind _currentdialoguerow (Variables|Default|GetCurrentDialogueRow))
  (bind (_rownumber _character _dialoguelong _nextrow _haschoice) (Utilities|Struct|BreakST_DialogueRowDatas _currentdialoguerow))
  (return (and (< _nextrow 0) (not _haschoice))))

(fn ReadNextRow
  (Variables|Default|SetCurrentRowNumber (.NextRow (Utilities|Struct|BreakST_DialogueRowDatas (Variables|Default|GetCurrentDialogueRow))))
  (CallFunction|GetCurrentDialogueRowData))

(fn GetChoiceData
  (bind _currentdialoguerow (Variables|Default|GetCurrentDialogueRow))
  (bind (_rownumber _character _dialoguelong _nextrow _haschoice _choicetext _choice1nextrow _choice1effect _choice2text _choice2nextrow _choice2effect) (Utilities|Struct|BreakST_DialogueRowDatas _currentdialoguerow))
  (return _haschoice _choicetext _choice1nextrow _choice1effect _choice2text _choice2nextrow _choice2effect))