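; Manager for the hide-and-seek minigame, which shows a tutorial on start and runs the round through to its reward.
; The game instance's mode picks whether the player or BP_ZombieNPC hides, with a timed cooldown widget or black screen for the hiding phase.
; A timed round follows, and expiry reports result 1.
; GameFinished adds gold for result 1, otherwise deducts it, then saves and opens the LoopHero level.
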(event Custom|StartHideAndSeekSequence
  (bind _asbp_loop_game_instance (Utilities|Casting|CastToBP_LoopGameInstance (Game|GetGameInstance)))
  (if (== (Variables|/Game/Blueprints/Global/BP_LoopGameInstance.BP_LoopGameInstance_C|GetHideAndSeekMode _asbp_loop_game_instance) 0)
    (bind _returnvalue (Actor|GetActorOfClass "/Game/Blueprints/Gameplay/Enemy/BP_ZombieNPC.BP_ZombieNPC_C"))
    (Variables|/Game/Blueprints/Gameplay/Enemy/BP_ZombieNPC.BP_ZombieNPC_C|SetIsHiding? _returnvalue false)
    (CallFunction|PlayerHide)
    (else
      (bind _returnvalue_2 (Actor|GetActorOfClass "/Game/Blueprints/Gameplay/Enemy/BP_ZombieNPC.BP_ZombieNPC_C"))
      (Variables|/Game/Blueprints/Gameplay/Enemy/BP_ZombieNPC.BP_ZombieNPC_C|SetIsHiding? _returnvalue_2 true)
      (CallFunction|AIHide))))

(event Custom|PlayerHide
  (bind _returnvalue (Game|GetPlayerController 0))
  (Input|EnableInput (Variables|Default|GetPlayerPawnRef) _returnvalue)
  (Variables|/Script/Engine.PlayerController|SetbShowMouseCursor _returnvalue false)
  (bind _returnvalue_2 (UserInterface|CreateWidget "/Game/Blueprints/Global/Widget/WBP_Cooldown.WBP_Cooldown_C" _returnvalue))
  (bind _output_get (Variables|Default|SetCooldownWidget _returnvalue_2))
  (UserInterface|Viewport|AddtoViewport _output_get 0)
  (Utilities|Time|SetTimerbyFunctionName 0 "OnHidePhaseFinished" 1e+01))

(event Custom|AIHide
  (bind _returnvalue (Game|GetPlayerController 0))
  (Input|DisableInput (Variables|Default|GetPlayerPawnRef) _returnvalue)
  (bind _returnvalue_2 (UserInterface|CreateWidget "/Game/Blueprints/Global/Widget/WBP_BlackScreen.WBP_BlackScreen_C" _returnvalue))
  (bind _output_get (Variables|Default|SetBSWidget _returnvalue_2))
  (UserInterface|Viewport|AddtoViewport _output_get 0)
  (Utilities|Time|SetTimerbyFunctionName 0 "OnBlackScreenEnd" 3.0))

(event Custom|StartTimer
  (Utilities|Time|ClearandInvalidateTimerbyHandle (Variables|Default|GetTimerHandle))
  (Variables|Default|SetTimerRemaining 4e+01)
  (Variables|Default|SetHideAndSeekActive true)
  (bind _returnvalue (Utilities|Time|SetTimerbyEvent (delegate Custom|TickRemainingTime) 1.0 true))
  (Variables|Default|SetTimerHandle _returnvalue)
  (bind _returnvalue_2 (UserInterface|CreateWidget "/Game/Blueprints/Global/Widget/WBP_Cooldown.WBP_Cooldown_C" (Game|GetPlayerController 0)))
  (bind _output_get (Variables|Default|SetCooldownWidget _returnvalue_2))
  (UserInterface|Viewport|AddtoViewport _output_get 0)
  (bind _returnvalue_3 (Utilities|Time|SetTimerbyFunctionName 0 "OnTimerExpired" 4e+01))
  (Variables|Default|SetTimerHandle _returnvalue_3))

(event Custom|GameFinished
  (params (Result :type Integer))
  (Variables|Default|SetHideAndSeekActive false)
  (Utilities|Time|ClearandInvalidateTimerbyHandle (Variables|Default|GetTimerHandle))
  (Variables|Default|SetTimerRemaining 0.0)
  (bind _asbp_loop_game_instance (Utilities|Casting|CastToBP_LoopGameInstance (Game|GetGameInstance)))
  (bind _output_get (Variables|/Game/Blueprints/Global/BP_LoopGameInstance.BP_LoopGameInstance_C|SetHideAndSeekResult _asbp_loop_game_instance Result))
  (if (== _output_get 1)
    (Variables|/Game/Blueprints/Global/BP_LoopGameInstance.BP_LoopGameInstance_C|SetPlayerGold _asbp_loop_game_instance (+ (Variables|/Game/Blueprints/Global/BP_LoopGameInstance.BP_LoopGameInstance_C|GetPlayerGold _asbp_loop_game_instance) 25))
    (bind _returnvalue (UserInterface|CreateWidget "/Game/Blueprints/Global/Widget/WBP_BlackScreen.WBP_BlackScreen_C" (Game|GetPlayerController 0)))
    (UserInterface|Viewport|AddtoViewport _returnvalue 100)
    (Default|PlayFadeOut _returnvalue)
    (Default|SaveGametoSlot _asbp_loop_game_instance)
    (Game|OpenLevel(byName) "LoopHero")
    (else
      (Variables|/Game/Blueprints/Global/BP_LoopGameInstance.BP_LoopGameInstance_C|SetPlayerGold _asbp_loop_game_instance (- (Variables|/Game/Blueprints/Global/BP_LoopGameInstance.BP_LoopGameInstance_C|GetPlayerGold _asbp_loop_game_instance) 30))
      (bind _returnvalue_2 (UserInterface|CreateWidget "/Game/Blueprints/Global/Widget/WBP_BlackScreen.WBP_BlackScreen_C" (Game|GetPlayerController 0)))
      (UserInterface|Viewport|AddtoViewport _returnvalue_2 100)
      (Default|PlayFadeOut _returnvalue_2)
      (Default|SaveGametoSlot _asbp_loop_game_instance)
      (Game|OpenLevel(byName) "LoopHero"))))

(event Custom|TickRemainingTime
  (if (Variables|Default|GetHideAndSeekActive)
    (bind _result (Math|Float|DecrementFloat (Variables|Default|GetTimerRemaining))
      (:%20%20
        (if (<= _result 0.0)
          _)))))

(event EventBeginPlay
  (bind _asbp_third_person_character (Utilities|Casting|CastToBP_ThirdPersonCharacter (Game|Player|GetPlayerPawn 0)))
  (bind _returnvalue (UserInterface|CreateWidget "/Game/Blueprints/Global/Widget/WBP_BlackScreen.WBP_BlackScreen_C" (Game|GetPlayerController 0)))
  (UserInterface|Viewport|AddtoViewport _returnvalue 100)
  (Default|PlayFadein _returnvalue)
  (Utilities|FlowControl|Delay 0.75)
  (Widget|RemovefromParent _returnvalue)
  (Utilities|FlowControl|Delay 1.0)
  (bind _output_get (Variables|Default|SetPlayerPawnRef _asbp_third_person_character))
  (bind _returnvalue_2 (UserInterface|CreateWidget "/Game/Blueprints/Global/Widget/WBP_TutoHideAndSeek.WBP_TutoHideAndSeek_C" (Game|GetPlayerController (Variables|/Script/Engine.Pawn|GetPlayerState _output_get))))
  (Variables|/Game/Blueprints/Global/Widget/WBP_TutoHideAndSeek.WBP_TutoHideAndSeek_C|SetMiniGameManagerRef _returnvalue_2 self)
  (UserInterface|Viewport|AddtoViewport _returnvalue_2 0)
  (Input|DisableInput (Game|GetPlayerController (Variables|/Script/Engine.Pawn|GetPlayerState _output_get)))
  (Variables|/Script/Engine.PlayerController|SetbShowMouseCursor (Game|GetPlayerController (Variables|/Script/Engine.Pawn|GetPlayerState _output_get)) true))

(event EventTick
  (params (DeltaSeconds :type Float%20%28single-precision%29)))

(fn ConstructionScript)

(fn OnHidePhaseFinished
  (Widget|RemovefromParent (Variables|Default|GetCooldownWidget))
  (CallFunction|StartTimer))

(fn OnBlackScreenEnd
  (bind _returnvalue (Game|GetPlayerController 0))
  (Widget|RemovefromParent (Variables|Default|GetBSWidget))
  (CallFunction|StartTimer)
  (Input|EnableInput _returnvalue)
  (Variables|/Script/Engine.PlayerController|SetbShowMouseCursor _returnvalue false))

(fn OnTimerExpired
  (if (Variables|Default|GetHideAndSeekActive)
    (CallFunction|GameFinished 1)))